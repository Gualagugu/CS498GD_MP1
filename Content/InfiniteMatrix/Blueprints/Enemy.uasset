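; Enemy is a spinning hazard actor that damages the player on contact and can be destroyed by projectiles.
; Tick rotates the root component on all three axes at a frame-rate-scaled Spin rate.
; Overlapping BP_Player subtracts a fixed amount of Health, writes the new percentage straight to the player's HUD and destroys the enemy.
; Overlapping a Prejectile destroys both actors.
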(event EventBeginPlay)

(event Collision|EventActorBeginOverlap
  (params (OtherActor :type Actor%20Object%20Reference))
  (Utilities|FlowControl|Sequence
    (:then_0
      (bind _asbp_player (Utilities|Casting|CastToBP_Player OtherActor))
      (bind _output_get (Variables|/Game/InfiniteMatrix/Blueprints/BP_Player.BP_Player_C|SetHealth _asbp_player (Math|Integer|Min(Integer) (+ (Variables|/Game/InfiniteMatrix/Blueprints/BP_Player.BP_Player_C|GetHealth _asbp_player) -30) 100)))
      (Variables|/Game/InfiniteMatrix/UI/HUD.HUD_C|Set%20HealthPercentage (Variables|/Game/InfiniteMatrix/Blueprints/BP_Player.BP_Player_C|GetHUD _asbp_player) (/ (Math|Conversions|ToFloat(Integer) _output_get) 1e+02))
      (Actor|DestroyActor))
    (:then_1
      (bind _asprejectile (Utilities|Casting|CastToPrejectile OtherActor))
      (Actor|DestroyActor)
      (Actor|DestroyActor _asprejectile))))

(event EventTick
  (params (DeltaSeconds :type Float%20%28single-precision%29))
  (bind _spin (Variables|Default|GetSpin))
  (bind _returnvalue (* DeltaSeconds _spin))
  (Class|SceneComponent|AddWorldTransform (Variables|Default|GetDefaultSceneRoot) (Math|Transform|MakeTransform "0.0,0.0,0.0" (Math|Rotator|MakeRotator _returnvalue _returnvalue _returnvalue) "1,1,1") false false))

(fn ConstructionScript)